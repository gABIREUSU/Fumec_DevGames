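; Ghost_BP is a short-lived Paper2D ghost actor that shows a tinted copy of a supplied flipbook and fades away.
; On BeginPlay it applies the SpriteToCopy flipbook and the Color tint to its sprite.
; A FadeOut timeline then drives the tint's alpha while keeping its RGB, and the actor destroys itself when the timeline finishes.
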(event EventBeginPlay
  (bind _sprite (Variables|Default|GetSprite))
  (bind _color (Variables|Default|GetColor))
  (bind (_r _g _b) (Math|Color|BreakColor _color))
  (Sprite|SetFlipbook _sprite (Variables|Default|GetSpriteToCopy))
  (Sprite|SetSpriteColor _sprite (Variables|Default|GetColor))
  (bind _alpha (Timeline|FadeOut Play)
    (:Update
      (Sprite|SetSpriteColor (Variables|Default|GetSprite) (Utilities|Struct|MakeLinearColor _r _g _b _alpha)))
    (:Finished
      (Actor|DestroyActor))))

(event Collision|EventActorBeginOverlap
  (params (OtherActor :type Actor%20Object%20Reference)))

(event EventTick
  (params (DeltaSeconds :type Float%20%28single-precision%29)))

(fn ConstructionScript)