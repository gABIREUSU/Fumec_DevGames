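; Game instance that holds run state across levels: stat buffs, enemy kill and stage counters, and the last level loaded.
; AbrirLevelAleatorio opens a random entry from Levels, re-rolling to avoid repeating the previous one.
; AtualizarStatus applies percent and flat buffs via CalcularBuff to the Player_BP's current damage, max health and speed.
; Reset zeroes the buffs and both counters, leaving the last-level index intact.
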(fn AbrirLevelAleatorio
  (bind _levels (Variables|Default|GetLevels))
  (bind _returnvalue (Utilities|Array|Length _levels))
  (bind _returnvalue_2 (- _returnvalue 1))
  (bind _returnvalue_3 (Math|Random|RandomIntegerinRange 0 _returnvalue_2))
  (if (== (Variables|Default|GetultimoLevel) -1)
    (bind _output_get (Variables|Default|SetIndex _returnvalue_3))
    (Variables|Default|SetultimoLevel _output_get)
    (Game|OpenLevel(byObjectReference) (Utilities|Array|Get(acopy) _levels _output_get))
    (else
      (while (== (Variables|Default|GetIndex) (Variables|Default|GetultimoLevel))
        (Variables|Default|SetIndex _returnvalue_3))
      (Variables|Default|SetultimoLevel (Variables|Default|GetIndex))
      (Game|OpenLevel(byObjectReference) (Utilities|Array|Get(acopy) _levels (Variables|Default|GetIndex))))))

(fn AtualizarStatus
  (bind _asplayer_bp (Utilities|Casting|CastToPlayer_BP (Game|Player|GetPlayerPawn 0)))
  (bind _returnvalue (CallFunction|CalcularBuff (Variables|/Game/Player/Blueprints/Player_BP.Player_BP_C|GetDano _asplayer_bp) (Variables|Default|GetAtaquePort) (Variables|Default|GetAtaqueFlat)))
  (Variables|/Game/Player/Blueprints/Player_BP.Player_BP_C|SetDano _asplayer_bp _returnvalue)
  (bind _returnvalue_2 (CallFunction|CalcularBuff (Variables|/Game/Player/Blueprints/Player_BP.Player_BP_C|GetVidaMaxima _asplayer_bp) (Variables|Default|GetVidaPort) (Variables|Default|GetVidaFlat)))
  (Variables|/Game/Player/Blueprints/Player_BP.Player_BP_C|SetVidaMaxima _asplayer_bp _returnvalue_2)
  (bind _returnvalue_3 (CallFunction|CalcularBuff (Variables|/Game/Player/Blueprints/Player_BP.Player_BP_C|GetVelocidade _asplayer_bp) (Variables|Default|GetVelocidadePort) (Variables|Default|GetVelocidadeFlat)))
  (Variables|/Game/Player/Blueprints/Player_BP.Player_BP_C|SetVelocidade _asplayer_bp _returnvalue_3))

(fn CalcularBuff
  (params (Status :type Float%20%28single-precision%29) (Porcentagem :type Float%20%28single-precision%29) (Flat :type Float%20%28single-precision%29))
  (return (+ (* Status (+ Porcentagem 1.0)) Flat)))

(fn Reset
  (Variables|Default|SetVelocidadeFlat 0.0)
  (Variables|Default|SetVelocidadePort 0.0)
  (Variables|Default|SetAtaqueFlat 0.0)
  (Variables|Default|SetAtaquePort 0.0)
  (Variables|Default|SetVidaFlat 0.0)
  (Variables|Default|SetVidaPort 0.0)
  (Variables|Default|SetNInimigosMortos 0)
  (Variables|Default|SetNFases 0))