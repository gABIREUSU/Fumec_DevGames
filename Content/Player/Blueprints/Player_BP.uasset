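; Side-scrolling 2D player character with run, jump, dash and combo attack, plus HUD, pause menu and level-exit fades.
; Velocity and actions set EstadoPlayer, which selects the sprite flipbook.
; Combo attacks enable the hit collision for roughly the flipbook's length, damaging overlapped InimigoBaseBP enemies.
; Tick clamps the spring arm within camera bounds; death and level-up are empty stubs, and a test input drains health.
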(event OnComponentBeginOverlap(Colisao)
  (params (OverlappedComponent :type Primitive%20Component%20Object%20Reference) (OtherActor :type Actor%20Object%20Reference) (OtherComp :type Primitive%20Component%20Object%20Reference) (OtherBodyIndex :type Integer) (bFromSweep :type Boolean) (SweepResult :type Hit%20Result%20Structure%20%28by%20ref%29))
  ;[1 1 1] Dano
  (if (Actor|ActorHasTag OtherActor "InimigoP")
    _
    (else
      _))
  (bind _asinimigo_base_bp (Utilities|Casting|CastToInimigoBaseBP OtherActor))
  (Default|TakeDamage _asinimigo_base_bp (Variables|Default|GetDano)))

(event Custom|GotoLevel
  (params (Fase :type Name))
  (bind _foundwidgets (Widget|GetAllWidgetsOfClass "/Game/Player/Blueprints/HUD/HUD_Padrao.HUD_Padrao_C" true))
  (bind _ashud_padrao (Utilities|Casting|CastToHUD_Padrao (Utilities|Array|Get(acopy) _foundwidgets)))
  (bind _outactors (Actor|GetAllActorsOfClass "/Game/Audios/AudioActor.AudioActor_C"))
  (bind _asaudio_actor (Utilities|Casting|CastToAudioActor (Utilities|Array|Get(acopy) _outactors)))
  (Default|FadeOUT _asaudio_actor)
  (Default|FadeOUT _ashud_padrao Fase))

(event EventBeginPlay
  ;[1 1 1] Hud Padrão
  (bind _returnvalue (UserInterface|CreateWidget "/Game/Player/Blueprints/HUD/HUD_Padrao.HUD_Padrao_C"))
  (UserInterface|Viewport|AddtoViewport _returnvalue 0)
  (Default|FadeIN _returnvalue))

(event EventTick
  (params (DeltaSeconds :type Float%20%28single-precision%29))
  (Utilities|LimitadorDeCamera)
  (if (not (Variables|Default|GetIsAttacking))
    (CallFunction|AnimMovimento)
    (CallFunction|UpdateAnimation)
    (if (< (Variables|Default|GetVidaAtual) 0.0)
      (Variables|Default|SetVidaAtual 0.0))))

(event Input|ActionEvents|InputActionPular
  (params (Key :type Key%20Structure :default "None"))
  ;[1 1 1] Pulo
  (:Pressed
    (Character|Jump))
  (:Released
    (Character|StopJumping)))

(event Input|ActionEvents|InputActionDireita
  (params (Key :type Key%20Structure :default "None"))
  ;[1 1 1] Movimentação
  (:Pressed
    (Variables|Default|SetIsMovingRight true)
    (Variables|Default|SetLastDirection (Variables|Default|GetVelocidadeMovimentoFinal)))
  (:Released
    (Variables|Default|SetIsMovingRight false)))

(event Input|ActionEvents|InputActionEsquerda
  (params (Key :type Key%20Structure :default "None"))
  ;[1 1 1] Movimentação
  (:Pressed
    (Variables|Default|SetIsMovingLeft true)
    (Variables|Default|SetLastDirection (* -1 (Variables|Default|GetVelocidadeMovimentoFinal))))
  (:Released
    (Variables|Default|SetIsMovingLeft false)))

(event Input|ActionEvents|InputActionAcaoTeste
  (params (Key :type Key%20Structure :default "None"))
  (:Pressed
    (Variables|Default|SetVidaAtual (- (Variables|Default|GetVidaAtual) 5.0))))

(event Input|ActionEvents|InputActionAtaque
  (params (Key :type Key%20Structure :default "None"))
  ;[1 1 1] Attack
  (:Pressed
    (Utilities|AtacarCombo)))

(event Input|ActionEvents|InputActionDash
  (params (Key :type Key%20Structure :default "None"))
  ;[1 1 1] Dash
  (:Pressed
    (if (Variables|Default|GetCanDash)
      (Variables|Default|SetCanDash false)
      (Variables|Default|SetEstadoPlayer "NewEnumerator6")
      (CallFunction|UpdateAnimation)
      (Character|LaunchCharacter (Math|Vector|MakeVector (* (Variables|Default|GetLastDirection) (Variables|Default|GetForcaDash)) 0.0 0.0) false true)
      (Variables|Default|SetCanDash true))))

(event Input|ActionEvents|InputActionPause
  (params (Key :type Key%20Structure :default "None"))
  (bind _returnvalue (Game|GetPlayerController 0))
  ;[1 1 1] Menus
  (:Pressed
    (CallFunction|GetMenuAtual)
    (if (Game|IsGamePaused)
      (Game|SetGamePaused false)
      (Widget|RemovefromParent (Variables|Default|GetMenuPause))
      (Input|SetInputModeGameOnly _returnvalue)
      (Variables|/Script/Engine.PlayerController|SetbShowMouseCursor _returnvalue false)
      (else
        (bind _returnvalue_2 (UserInterface|CreateWidget (Variables|Default|GetClass)))
        (Variables|Default|SetMenuPause _returnvalue_2)
        (UserInterface|Viewport|AddtoViewport (Variables|Default|GetMenuPause) 0)
        (Input|SetInputModeGameandUI _returnvalue 0 "DoNotLock" true)
        (Game|SetGamePaused true)
        (Variables|/Script/Engine.PlayerController|SetbShowMouseCursor _returnvalue true)))
    (bind _outactors (Actor|GetAllActorsOfClass "/Game/Audios/AudioActor.AudioActor_C"))
    (bind _asaudio_actor (Utilities|Casting|CastToAudioActor (Utilities|Array|Get(acopy) _outactors)))
    (Default|TransicaoMenu _asaudio_actor)))

(event Input|AxisEvents|InputAxisMoverLados
  (params (AxisValue :type Float%20%28single-precision%29))
  (bind _ismovingright (Variables|Default|GetIsMovingRight))
  (bind _sprite (Variables|Default|GetSprite))
  (bind _velocidademovimentofinal (Variables|Default|GetVelocidadeMovimentoFinal))
  (bind _returnvalue (* -1 _velocidademovimentofinal))
  ;[1 1 1] Movimentação
  (if (Variables|Default|GetIsMovingLeft)
    (if _ismovingright
      (Variables|Default|SetDirecao (Variables|Default|GetLastDirection))
      (else
        (Variables|Default|SetDirecao _returnvalue)))
    (elif _ismovingright
      (Variables|Default|SetDirecao _velocidademovimentofinal)
      (else
        (Variables|Default|SetDirecao 0.0))))
  (Pawn|Input|AddMovementInput "1.000000,0.000000, 0" (Variables|Default|GetDirecao) false)
  (if (== (Variables|Default|GetDirecao) _returnvalue)
    (Transformation|SetRelativeScale3D _sprite "-1.000000,1.000000,1.000000")
    (elif (== (Variables|Default|GetDirecao) _velocidademovimentofinal)
      (Transformation|SetRelativeScale3D _sprite "1.000000,1.000000,1.000000"))))

(fn ConstructionScript)

(fn UpdateAnimation
  (bind _sprite (Variables|Default|GetSprite))
  (switch Utilities|FlowControl|Switch|SwitchonEstadoPlayer (Variables|Default|GetEstadoPlayer)
    (:NewEnumerator0
      (Sprite|SetFlipbook _sprite "/Game/Player/Sprites/Animacoes/Idle.Idle"))
    (:NewEnumerator1
      (Sprite|SetFlipbook _sprite "/Game/Player/Sprites/Animacoes/Run.Run"))
    (:NewEnumerator2
      (Sprite|SetFlipbook _sprite "/Game/Player/Sprites/Animacoes/Attack1.Attack1"))
    (:NewEnumerator4
      (Sprite|SetFlipbook _sprite "/Game/Player/Sprites/Animacoes/Attack2.Attack2"))
    (:NewEnumerator5
      (Sprite|SetFlipbook _sprite "/Game/Player/Sprites/Animacoes/Attack3.Attack3"))
    (:NewEnumerator6
      (Sprite|SetFlipbook _sprite "/Game/Player/Sprites/Animacoes/Dash.Dash"))
    (:NewEnumerator7
      (Sprite|SetFlipbook _sprite "/Game/Player/Sprites/Animacoes/Defeat.Defeat"))
    (:NewEnumerator8
      (Sprite|SetFlipbook _sprite "/Game/Player/Sprites/Animacoes/Fall.Fall"))
    (:NewEnumerator9
      (Sprite|SetFlipbook _sprite "/Game/Player/Sprites/Animacoes/Hit.Hit"))
    (:NewEnumerator10
      (Sprite|SetFlipbook _sprite "/Game/Player/Sprites/Animacoes/Jump.Jump"))
    (:NewEnumerator11
      (Sprite|SetFlipbook _sprite "/Game/Player/Sprites/Animacoes/Transform.Transform"))))

(fn AnimMovimento
  (bind _returnvalue (Transformation|GetVelocity))
  (bind _charactermovement (Variables|Character|GetCharacterMovement))
  (bind _returnvalue_2 (AI|Components|NavMovement|IsFalling _charactermovement))
  (if (> (.z _returnvalue) 0.1)
    (if _returnvalue_2
      (Variables|Default|SetEstadoPlayer "NewEnumerator10")
      (else
        (if (!= (.x _returnvalue) 0.0) :!label _label
          (Variables|Default|SetEstadoPlayer "NewEnumerator1")
          (else
            (Variables|Default|SetEstadoPlayer "NewEnumerator0")))))
    (elif (< (.z _returnvalue) -0.1)
      (if _returnvalue_2
        (Variables|Default|SetEstadoPlayer "NewEnumerator8")
        (else
          (goto _label)))
      (else
        (goto _label)))))

(fn Morrer)

(fn SubirDeNivel)

(fn GetMenuAtual
  (bind _returnvalue (Game|GetCurrentLevelName true))
  (if (Utilities|Enum|Equal(Enum) _returnvalue "MapaInicial")
    (Variables|Default|SetClass "/Game/Player/Blueprints/HUD/MenuPauseInicio/MenuPauseInicio.MenuPauseInicio_C")
    (else
      (Variables|Default|SetClass "/Game/Player/Blueprints/HUD/MenuPausePadrao.MenuPausePadrao_C"))))